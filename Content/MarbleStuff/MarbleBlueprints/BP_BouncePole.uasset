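; BP_BouncePole is a pinball-style bumper actor that bounces marbles and awards points.
; When a BP_Marble overlaps its capsule, it applies an acceleration-change force along the normalized marble-to-pole vector, scaled by BounceForce.
; It then spawns a hit particle at EffuSphere, plays a quiet 2D bounce sound, and adds points to PlayerPoints in MarbleGameMode.
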(event `self.CapsuleCollision.OnComponentBeginOverlap`
  (params (OverlappedComponent :type "PrimitiveComponent Object Reference") (OtherActor :type "Actor Object Reference") (OtherComp :type "PrimitiveComponent Object Reference") (OtherBodyIndex :type Integer) (bFromSweep :type Boolean) (SweepResult :type "HitResult Structure (by ref)"))
  ;[1 1 1] Bounce Logic
  (bind _asbp_marble (cast `/Game/MarbleStuff/MarbleBlueprints/BP_Marble` OtherActor))
  (`PrimitiveComponent.AddForce` (`/Game/MarbleStuff/MarbleBlueprints/BP_Marble.MarbleSphere` _asbp_marble) (* (`KismetMathLibrary.Normal` (- (`self.K2_GetActorLocation`) (`SceneComponent.K2_GetComponentLocation` (`/Game/MarbleStuff/MarbleBlueprints/BP_Marble.MarbleSphere` _asbp_marble)))) (`self.BounceForce`)) "None" true)
  (`GameplayStatics.SpawnEmitterAtLocation` "/Game/FXVarietyPack/Particles/P_ky_waterBallHit.P_ky_waterBallHit" (`KismetMathLibrary.MakeVector` (.x (`SceneComponent.K2_GetComponentLocation` (`self.EffuSphere`))) (.y (`SceneComponent.K2_GetComponentLocation` (`self.EffuSphere`))) (.z (`SceneComponent.K2_GetComponentLocation` (`self.EffuSphere`)))))
  (`GameplayStatics.PlaySound2D` "/Game/Assets/BouncePole/523088__magnuswaker__energy-bounce-1.523088__magnuswaker__energy-bounce-1" 0.1 1.0 0.0 null null)
  (bind _asmarble_game_mode (cast `/Game/PlayerController/MarbleGameMode` (`GameplayStatics.GetGameMode`)))
  (set `/Game/PlayerController/MarbleGameMode.PlayerPoints` (+ (`/Game/PlayerController/MarbleGameMode.PlayerPoints` _asmarble_game_mode) 10) _asmarble_game_mode))

(fn `UserConstructionScript`)