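; BP_Marble is a marble that the player fires with a charged Space bar launch.
; Beginning any sphere overlap enables input and adds a charge bar widget before the launcher cast, while leaving a BP_MarbleLauncher disables input.
; Holding Space builds a clamped charge on Tick, exposed through GetCharge.
; Release applies a mass-independent force along a tilted up vector, interpolated between minimum and maximum by charge.
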(event `Key|SpaceBar`
  (params (Key :type "Key Structure"))
  (:`Pressed`
    (set `self.LaunchKeyDown?` true)
    (set `self.LaunchCharge` 0.0))
  (:`Released`
    (set `self.LaunchKeyDown?` false)
    (`self.PerformLaunch`)))

(event `self.ReceiveTick`
  (params (DeltaSeconds :type "Float (single-precision)"))
  (`self.TickLaunch` DeltaSeconds))

(event `self.Sphere.OnComponentBeginOverlap`
  (params (OverlappedComponent :type "PrimitiveComponent Object Reference") (OtherActor :type "Actor Object Reference") (OtherComp :type "PrimitiveComponent Object Reference") (OtherBodyIndex :type Integer) (bFromSweep :type Boolean) (SweepResult :type "HitResult Structure (by ref)"))
  (bind _returnvalue (`GameplayStatics.GetPlayerController` 0))
  (`self.EnableInput` _returnvalue)
  (bind _returnvalue_2 (`|CreateWidget` "/Game/MarbleStuff/UI/UI_MarbleChargeBar.UI_MarbleChargeBar_C" _returnvalue))
  (`UserWidget.AddToViewport` _returnvalue_2 0)
  (cast `/Game/MarbleStuff/MarbleBlueprints/BP_MarbleLauncher` OtherActor))

(event `self.Sphere.OnComponentEndOverlap`
  (params (OverlappedComponent :type "PrimitiveComponent Object Reference") (OtherActor :type "Actor Object Reference") (OtherComp :type "PrimitiveComponent Object Reference") (OtherBodyIndex :type Integer))
  (cast `/Game/MarbleStuff/MarbleBlueprints/BP_MarbleLauncher` OtherActor)
  (`self.DisableInput` (`GameplayStatics.GetPlayerController` 0)))

(fn `GetCharge`
  (returns (LaunchCharge :type "Float (double-precision)"))
  (return (`self.LaunchCharge`)))

(fn `PerformLaunch`
  (`PrimitiveComponent.AddForce` (`self.Sphere`) (* (`KismetMathLibrary.RotateAngleAxis` (`KismetMathLibrary.Vector_Up`) -35.0 (0.0 1.0 0.0)) (`KismetMathLibrary.Lerp` (`self.MinChargeVelocity`) (`self.MaxChargeVelocity`) (`self.LaunchCharge`))) "None" true)
  (set `self.LaunchCharge` 0.0))

(fn `TickLaunch`
  (params (DeltaSeconds :type "Float (double-precision)"))
  (if (`self.LaunchKeyDown?`)
    (set `self.LaunchCharge` (`KismetMathLibrary.FClamp` (+ (`self.LaunchCharge`) (/ (`local.DeltaSeconds`) (`self.ChargeTime`)))))))

(fn `UserConstructionScript`)