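; BP_Pointbox is a scoring box for the marble game that awards points when a marble enters it.
; When a BP_Marble overlaps its Box component, it destroys the marble and passes its BoxScorePoints to AddPoints on the MarbleGameMode.
; Leftover unconnected nodes from earlier scoring attempts remain in the graph but never run.
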(event `self.Box.OnComponentBeginOverlap`
  (params (OverlappedComponent :type "PrimitiveComponent Object Reference") (OtherActor :type "Actor Object Reference") (OtherComp :type "PrimitiveComponent Object Reference") (OtherBodyIndex :type Integer) (bFromSweep :type Boolean) (SweepResult :type "HitResult Structure (by ref)"))
  (bind _asbp_marble (cast `/Game/MarbleStuff/BP_Marble` OtherActor))
  (`self.K2_DestroyActor` _asbp_marble)
  (bind _asmarble_game_mode (cast `/Game/PlayerController/MarbleGameMode` (`GameplayStatics.GetGameMode`)))
  (`/Game/PlayerController/MarbleGameMode.AddPoints` _asmarble_game_mode (`self.Box Score Points`)))

(fn `UserConstructionScript`)